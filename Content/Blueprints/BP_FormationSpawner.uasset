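; Formation spawner actor that fills a grid of rows and columns with AI or player-less units when play begins.
; Each slot spawns a controller and a unit of the configured classes, then has the controller possess the unit.
; Slots follow the spawner's rotation, spreading along its right vector around its location, with later rows stepping backward.
; GetSpawnXStartPos computes a world-X start offset but is not called here.
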(event `self.ReceiveBeginPlay`
  (bind _returnvalue (`KismetMathLibrary.MakeTransform` (`self.CurrSpawnLoc`) (`self.K2_GetActorRotation`)))
  (set `self.CurrSpawnLoc` (- (`self.K2_GetActorLocation`) (* (`self.GetActorRightVector`) (* (/ (- (`self.Cols`) 1) 2) (`self.Spacing`)))))
  (for _ (range (`self.Rows`))
    (for _ (range (`self.Cols`))
      (bind _returnvalue_2 (`|SpawnActorFromClass` (`self.ControllerToAssign`) _returnvalue "AlwaysSpawn" "OverrideRootScale" null null))
      (bind _returnvalue_3 (`|SpawnActorFromClass` (`self.UnitToSpawn`) _returnvalue "AlwaysSpawn" "OverrideRootScale" null null))
      (`Controller.Possess` _returnvalue_2 _returnvalue_3)
      (set `self.CurrSpawnLoc` (+ (`self.CurrSpawnLoc`) (* (`self.GetActorRightVector`) (`self.Spacing`)))))
    (set `self.CurrSpawnLoc` (- (- (`self.CurrSpawnLoc`) (* (`self.GetActorForwardVector`) (`self.Spacing`))) (* (`self.GetActorRightVector`) (* (`self.Spacing`) (`self.Cols`)))))))

(fn `GetSpawnXStartPos`
  (returns (StartXPos :type "Float (double-precision)"))
  (bind _returnvalue_x (`KismetMathLibrary.BreakVector` (`self.K2_GetActorLocation`)))
  (return (- _returnvalue_x (* (`KismetMathLibrary.Conv_IntToDouble` (- (`self.Cols`) 1)) (`self.Spacing`)))))

(fn `UserConstructionScript`)