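; Test flow field grid actor that spawns a grid of FlowFieldCell actors from its location on BeginPlay.
; SpawnCells fills the Cells array row by row, deriving cell spacing and overall grid extents from the first spawned cell's extent.
; Helpers convert between flat indices and X/Y coordinates.
; GetNeighbors is an unfinished stub, and no flow direction computation exists yet.
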(event `self.ReceiveBeginPlay`
  (`self.SpawnCells`))

(event `Key|SpaceBar`
  (params (Key :type "Key Structure")))

(fn `GetNeighbors`
  (params (Index :type Integer))
  (returns (Neighbors :type "Array of /Game/Blueprints/TEST_Cell Object Reference"))
  (locals (MyPosX :type Integer) (MyPosY :type Integer) (MyNeighbors :type "Array of /Game/Blueprints/TEST_Cell Object Reference"))
  (bind (_x _y) (`self.IndexToPos` Index))
  (`|ExecutionSequence`
    (:`then_0`
      (set `local.MyPosX` _x)
      (set `local.MyPosY` _y))
    (:`then_1`
      (`|ExecutionSequence`
        (:`then_0`
          (if (>= (- (`local.MyPosX`) 1) 0)
            _))))
    (:`then_2`
      (return (`local.MyNeighbors`)))))

(fn `IndexToPos`
  (params (Index :type Integer))
  (returns (X :type Integer) (Y :type Integer))
  (return (mod Index (`self.GridWidth`)) (/ Index (`self.GridWidth`))))

(fn `PosToIndex`
  (params (X :type Integer) (Y :type Integer))
  (returns (Index :type Integer))
  (return (+ X (* Y (`self.GridWidth`)))))

(fn `SpawnCells`
  (locals (StartSpawnPos :type "Vector Structure") (SpawnPos :type "Vector Structure") (CellStep :type "Vector Structure" :default (0.0 0.0 0.0)))
  (bind (_cellstep_x _cellstep_y) (`KismetMathLibrary.BreakVector` (`local.CellStep`)))
  (bind (_startspawnpos_x _startspawnpos_y _startspawnpos_z) (`KismetMathLibrary.BreakVector` (`local.StartSpawnPos`)))
  (bind (_cellstep_x_2 _cellstep_y_2) (`KismetMathLibrary.BreakVector` (`local.CellStep`)))
  (bind (_spawnpos_x _spawnpos_y) (`KismetMathLibrary.BreakVector` (`local.SpawnPos`)))
  (bind _cellstep_x_3 (`KismetMathLibrary.BreakVector` (`local.CellStep`)))
  (bind _output_get (set `local.StartSpawnPos` (+ (`self.K2_GetActorLocation`) (50.0 50.0 0.0))))
  (set `local.SpawnPos` _output_get)
  (for _ (range (`self.GridHeight`))
    (for _ (range (`self.GridWidth`))
      (bind _returnvalue (`|SpawnActorFromClass` (`self.FlowFieldCell`) (`KismetMathLibrary.Conv_VectorToTransform` (`local.SpawnPos`)) "Undefined" "OverrideRootScale" null null))
      (`KismetArrayLibrary.Array_Add` (`self.Cells`) _returnvalue)
      (`|ExecutionSequence`
        (:`then_0`
          (`/Engine/EditorBlueprintResources/StandardMacros.DoOnce` false
            (:`Completed`
              (set `local.CellStep` (* (`/Game/Blueprints/TEST_Cell.GetCellExtent` _returnvalue) 2.0))
              (set `self.GridExtents` (`KismetMathLibrary.MakeVector` (* _cellstep_x_2 (`self.GridWidth`)) (* _cellstep_y_2 (`self.GridHeight`)) 200.0)))))
        (:`then_1`
          (set `local.SpawnPos` (+ (`local.SpawnPos`) (`KismetMathLibrary.MakeVector` _cellstep_x_3))))))
    (set `local.SpawnPos` (`KismetMathLibrary.MakeVector` _startspawnpos_x (+ _spawnpos_y _cellstep_y) _startspawnpos_z))))

(fn `UserConstructionScript`)