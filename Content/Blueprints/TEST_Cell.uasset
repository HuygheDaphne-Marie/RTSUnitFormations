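; Grid cell test Blueprint that determines whether the space it occupies is walkable.
; On BeginPlay it runs a zero-length multi box trace on the Visibility channel, sized to its CellCollision box, and sets IsWalkable when nothing blocks.
; A toggle function colors DebugVisual by walkable status and flips its in-game visibility.
; A getter exposes the cell's box extent.
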(event `self.ReceiveBeginPlay`
  (bind _cell_collision (`self.Cell Collision`))
  (bind _returnvalue (`SceneComponent.K2_GetComponentLocation` _cell_collision))
  ;[1 1 1] Check if Walkable
  (bind (_outhits _returnvalue_2) (`KismetSystemLibrary.BoxTraceMulti` _returnvalue _returnvalue (`BoxComponent.BoxExtent` _cell_collision) (struct) "TraceTypeQuery1"))
  (set `self.IsWalkable` (not _returnvalue_2)))

(fn `GetCellExtent`
  (returns (`Cell Extent` :type "Vector Structure"))
  (return (`BoxComponent.BoxExtent` (`self.Cell Collision`))))

(fn `ToggleShow Debug Walkable Status`
  (locals (WalkableMat :type "MaterialInstance Object Reference" :default "MaterialInstanceConstant'/Game/Materials/Debug/MI_Green.MI_Green'") (NotWalkableMat :type "MaterialInstance Object Reference" :default "MaterialInstanceConstant'/Game/Materials/Debug/MI_Red.MI_Red'"))
  (bind _debug_visual (`self.Debug Visual`))
  (`PrimitiveComponent.SetMaterial` (`self.Debug Visual`) 0 (select `bool` (`self.IsWalkable`) :`false` (`local.NotWalkableMat`) :`true` (`local.WalkableMat`)))
  (`SceneComponent.SetHiddenInGame` _debug_visual (not (`SceneComponent.bHiddenInGame` _debug_visual)) true))

(fn `UserConstructionScript`)